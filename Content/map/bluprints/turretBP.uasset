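; Turret actor that turns to a Target and fires BulletBP projectiles from its FirePoint.
; Each Tick computes and prints Distance as the difference between the turret's and target's distances from world origin, not their separation.
; Within a fixed band, it sets yaw from the target's normalized world position, ignoring its own location, and spawns a bullet.
; A CanShoot flag, re-armed by a Delay in Tick, limits the fire rate.
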(event Custom|DistanceCalculate
  (bind _returnvalue (Transformation|GetActorLocation))
  (bind _target (Variables|Default|Gettarget))
  (bind _returnvalue_2 (Transformation|GetActorLocation _target))
  (bind _output_get (Variables|Default|Setdistance (- (Math|Float|Sqrt (|(((x*x)+(y*y))+(z*z)) (.x _returnvalue) (.y _returnvalue) (.z _returnvalue))) (Math|Float|Sqrt (|(((x*x)+(y*y))+(z*z)) (.x _returnvalue_2) (.y _returnvalue_2) (.z _returnvalue_2))))))
  (Development|PrintString (Utilities|String|ToString(Float) _output_get)))

(event Custom|TargetLock
  (bind _target (Variables|Default|Gettarget))
  (Utilities|IsValid _target
    (:Is%20Valid
      (Transformation|SetActorRotation (Math|Rotator|MakeRotator 0.0 0.0 (.yaw (Math|Conversions|RotationFromXVector (Math|Vector|Normalize (Transformation|GetActorLocation _target)))))))))

(event Custom|SpawnBullet
  (if (Variables|Default|GetcanShoot)
    (Game|SpawnActorfromClass "/Game/map/bluprints/BulletBP.BulletBP_C" (Transformation|GetWorldTransform (Variables|Default|GetFirePoint)) "Undefined" 0 0)
    (Variables|Default|SetcanShoot false)))

(event EventBeginPlay)

(event Collision|EventActorBeginOverlap
  (params (OtherActor :type Actor%20Object%20Reference)))

(event EventTick
  (params (DeltaSeconds :type Float%20%28single-precision%29))
  (bind _distance (Variables|Default|Getdistance))
  (CallFunction|DistanceCalculate)
  (Math|Float|CompareFloat _distance 5e+02
    (:<
      (Math|Float|CompareFloat _distance -5e+02
        (:>
          (CallFunction|TargetLock)
          (CallFunction|SpawnBullet)
          (Utilities|FlowControl|Delay 4.0)
          (Variables|Default|SetcanShoot true))))))

(fn ConstructionScript)